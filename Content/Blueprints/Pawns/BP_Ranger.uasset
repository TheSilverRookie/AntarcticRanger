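; Player character pawn for a shooter, handling movement, look, aim-down-sights, health, death fade to the main menu, and kill and crystal counters.
; Firing is gated by fire rate plus clip or heat checks, then passes a camera-based trace to the equipped gun.
; Weapon swapping cycles owned guns by destroying and respawning the actor, saving and restoring ammo and heat.
; Debug keys for self-damage and free ammo remain wired.
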(event `InputAction|Reload`
  (params (Key :type "Key Structure"))
  (bind _equippedgun (`self.EquippedGun`))
  (:`Pressed`
    (if (`self.IsAlive`)
      (if (!= (`/Game/Blueprints/Actors/Guns/BP_GunParent.AmmoCount` _equippedgun) 0)
        (if (`/Game/Blueprints/Actors/Guns/BP_GunParent.IsHeatBased` _equippedgun)
          (`/Game/Blueprints/Actors/Guns/BP_GunParent.ManualCooldown` _equippedgun)
          (else
            (`/Game/Blueprints/Actors/Guns/BP_GunParent.Reload` _equippedgun)))))))

(event `InputAction|AimDownSight`
  (params (Key :type "Key Structure"))
  ;[1 1 1] Aim Down Sights
  (:`Pressed`
    (`/Engine/EditorBlueprintResources/StandardMacros.FlipFlop` :!label _label
      (:`A`
        (`self.DecreaseMovementSpeed`)
        (bind (_direction _adsmove) (`Timeline|ADS_Timeline` :!label _label_2)
          (:`Update`
            (`self.ToggleCameraPosition` _adsmove))))
      (:`B`
        (`self.IncreaseMovementSpeed`)
        (goto _label_2 :!via `Reverse`))))
  (:`Released`
    (goto _label)))

(event `Key|F`
  (params (Key :type "Key Structure"))
  ;[1 1 1] Debug - BREAK LINKS FOR BUILDS!
  (:`Pressed`
    (`GameplayStatics.ApplyDamage` self 25.0)))

(event `self.ReceiveAnyDamage`
  (params (Damage :type "Float (single-precision)") (DamageType :type "DamageType Object Reference") (InstigatedBy :type "Controller Object Reference") (DamageCauser :type "Actor Object Reference"))
  ;[1 1 1] When the Player takes Damage
  (if (`self.IsAlive`)
    (bind _health (`self.DecreaseHealth` Damage))
    (if (== _health 0.0)
      (set `self.Dead` true)
      (`self.DisableInput` (`GameplayStatics.GetPlayerController` 0))
      (`PlayerCameraManager.StartCameraFade` :`self` (`GameplayStatics.GetPlayerCameraManager` 0) :`ToAlpha` 1.0 :`Duration` 2.0 :`bHoldWhenFinished` true)
      (`KismetSystemLibrary.Delay` 2.5)
      (`GameplayStatics.OpenLevel` "MainMenu"))))

(event `Key|Enter`
  (params (Key :type "Key Structure"))
  ;[1 1 1] Debug - BREAK LINKS FOR BUILDS!
  (:`Pressed`
    (`/Game/Blueprints/Actors/Guns/BP_GunParent.AddAmmo` (`self.EquippedGun`) 10)))

(event `InputAxis|LookUp`
  (params (AxisValue :type "Float (single-precision)"))
  ;[1 1 1] Looking
  (if (`self.IsAlive`)
    (`self.AddControllerPitchInput` AxisValue)))

(event `InputAxis|MoveForward`
  (params (AxisValue :type "Float (single-precision)"))
  ;[1 1 1] Movement
  (if (`self.IsAlive`)
    (`self.AddMovementInput` (`self.GetForwardDirection`) AxisValue)))

(event `self.ReceiveBeginPlay`
  ;[1 1 1] Initialisation
  (`self.SpawnPlayerWeapons`)
  (bind _returnvalue (`|CreateWidget` "/Game/Blueprints/Widgets/HUD.HUD_C" null self))
  (`UserWidget.AddToViewport` _returnvalue 0)
  (`PlayerCameraManager.StartCameraFade` :`self` (`GameplayStatics.GetPlayerCameraManager` 0) :`FromAlpha` 1.0 :`Duration` 2.0)
  (`WidgetBlueprintLibrary.SetInputMode_GameOnly` (`GameplayStatics.GetPlayerController` 0)))

(event `InputAxis|LookRight`
  (params (AxisValue :type "Float (single-precision)"))
  ;[1 1 1] Looking
  (if (`self.IsAlive`)
    (`self.AddControllerYawInput` AxisValue)))

(event `InputAxis|MoveRight`
  (params (AxisValue :type "Float (single-precision)"))
  ;[1 1 1] Movement
  (if (`self.IsAlive`)
    (`self.AddMovementInput` (`self.GetRightDirection`) AxisValue)))

(event `InputAction|SwapWeapon`
  (params (Key :type "Key Structure"))
  (:`Pressed`
    (`self.SwitchWeapon`)))

(event `InputAxis|FireWeapon`
  (params (AxisValue :type "Float (single-precision)"))
  ;[1 1 1] Firing Weapon
  (if (`self.IsAlive`)
    (if (`self.CanPlayerShoot` AxisValue)
      (if (`/Game/Blueprints/Actors/Guns/BP_GunParent.IsHeatBased` (`self.EquippedGun`))
        (if (`self.CanBeFired`)
          (`self.FireGun` :!label _label_3)
          (`self.SetGunHeat`)
          (set `self.CanShoot` false)
          (`KismetSystemLibrary.Delay` (`self.GetGunFireRate`))
          (set `self.CanShoot` true))
        (elif (not (`self.IsGunClipEmpty`))
          (goto _label_3))))))

(fn `CanBeFired`
  (returns (ReturnValue :type Boolean))
  (return (and (`self.IsGunNotOverheating`) (`self.IsThereAmmo`))))

(fn `CanPlayerShoot`
  (params (AxisValue :type "Float (double-precision)"))
  (returns (ReturnValue :type Boolean))
  (return (and (== AxisValue 1.0) (`self.CanShoot`))))

(fn `DecreaseHealth`
  (params (DamageAmount :type "Float (double-precision)"))
  (returns (Health :type "Float (double-precision)"))
  (bind _output_get (set `self.Health` (`KismetMathLibrary.FClamp` (- (`self.Health`) DamageAmount) 0.0 100.0)))
  (return _output_get))

(fn `DecreaseMovementSpeed`
  (bind _charactermovement (`self.CharacterMovement`))
  (set `CharacterMovementComponent.MaxWalkSpeed` (* (`CharacterMovementComponent.MaxWalkSpeed` _charactermovement) 0.5) _charactermovement))

(fn `FireGun`
  (if (`self.IsAlive`)
    (bind _bulletdirection (`self.SetBulletDirection`))
    (`/Game/Blueprints/Actors/Guns/BP_GunParent.FireGun` (`self.EquippedGun`) (`self.GetTraceStart`) (`self.GetTraceEnd`) _bulletdirection)))

(fn `Get ADS Location`
  (returns (ReturnValue :type "Vector Structure"))
  (return (`SceneComponent.K2_GetComponentLocation` (`/Game/Blueprints/Actors/Guns/BP_GunParent.ADS_Location` (`self.EquippedGun`)))))

(fn `GetCameraStartingLocation`
  (returns (ReturnValue :type "Vector Structure"))
  (return (`SceneComponent.K2_GetComponentLocation` (`self.MainCameraLocation`))))

(fn `GetCurrentAmmo`
  (params (WeaponClass :type "/Game/Blueprints/Actors/Guns/BP_GunParent Class Reference"))
  (returns (GunVariables :type "/Game/Blueprints/GunVariables Structure"))
  (bind _equippedgun (`self.EquippedGun`))
  (return (make `/Game/Blueprints/GunVariables` WeaponClass (`/Game/Blueprints/Actors/Guns/BP_GunParent.AmmoCount` _equippedgun) (`/Game/Blueprints/Actors/Guns/BP_GunParent.MaximumAmmo` _equippedgun) (`/Game/Blueprints/Actors/Guns/BP_GunParent.CurrentClip` _equippedgun) (`/Game/Blueprints/Actors/Guns/BP_GunParent.CurrentHeat` _equippedgun))))

(fn `GetForwardDirection`
  (returns (ReturnValue :type "Vector Structure"))
  (return (`KismetMathLibrary.GetForwardVector` (`CharacterMovementComponent.GetLastUpdateRotation` (`self.CharacterMovement`)))))

(fn `GetGunFireRate`
  (returns (FireRate :type "Float (double-precision)"))
  (return (`/Game/Blueprints/Actors/Guns/BP_GunParent.FireRate` (`self.EquippedGun`))))

(fn `GetRightDirection`
  (returns (ReturnValue :type "Vector Structure"))
  (return (`KismetMathLibrary.GetRightVector` (`CharacterMovementComponent.GetLastUpdateRotation` (`self.CharacterMovement`)))))

(fn `GetTraceEnd`
  (returns (ReturnValue :type "Vector Structure"))
  (return (+ (`self.GetTraceStart`) (* (`KismetMathLibrary.GetForwardVector` (`self.GetControlRotation`)) (`/Game/Blueprints/Actors/Guns/BP_GunParent.MaxBulletDistance` (`self.EquippedGun`))))))

(fn `GetTraceStart`
  (returns (ReturnValue :type "Vector Structure"))
  (return (`SceneComponent.K2_GetComponentLocation` (`self.Camera1`))))

(fn `IncreaseCrystal`
  (`/Engine/EditorBlueprintResources/StandardMacros.IncrementInt` (`self.Crystals`)))

(fn `IncreaseKillCount`
  (`/Engine/EditorBlueprintResources/StandardMacros.IncrementInt` (`self.KillCount`)))

(fn `IncreaseMovementSpeed`
  (bind _charactermovement (`self.CharacterMovement`))
  (set `CharacterMovementComponent.MaxWalkSpeed` (* (`CharacterMovementComponent.MaxWalkSpeed` _charactermovement) 2.0) _charactermovement))

(fn `IsAlive`
  (returns (ReturnValue :type Boolean))
  (return (not (`self.Dead`))))

(fn `IsGunClipEmpty`
  (returns (ReturnValue :type Boolean))
  (return (`/Game/Blueprints/Actors/Guns/BP_GunParent.IsCurrentClipEmpty` (`self.EquippedGun`))))

(fn `IsGunNotOverheating`
  (returns (ReturnValue :type Boolean))
  (return (not (`/Game/Blueprints/Actors/Guns/BP_GunParent.IsOverheated` (`self.EquippedGun`)))))

(fn `IsHealthFull`
  (returns (ReturnValue :type Boolean))
  (return (>= (`self.Health`) 100.0)))

(fn `IsThereAmmo`
  (returns (ReturnValue :type Boolean))
  (return (`/Game/Blueprints/Actors/Guns/BP_GunParent.IsThereAmmo` (`self.EquippedGun`))))

(fn `LoadSavedAmmo`
  (params (AmmoCount :type Integer) (MaximumAmmo :type Integer) (CurrentClip :type Integer) (CurrentHeat :type "Float (double-precision)"))
  (bind _equippedgun (`self.EquippedGun`))
  (set `/Game/Blueprints/Actors/Guns/BP_GunParent.AmmoCount` AmmoCount _equippedgun)
  (set `/Game/Blueprints/Actors/Guns/BP_GunParent.MaximumAmmo` MaximumAmmo _equippedgun)
  (set `/Game/Blueprints/Actors/Guns/BP_GunParent.CurrentClip` CurrentClip _equippedgun)
  (set `/Game/Blueprints/Actors/Guns/BP_GunParent.CurrentHeat` CurrentHeat _equippedgun))

(fn `RestoreHealth`
  (params (HealingAmount :type "Float (double-precision)"))
  (returns (Health :type "Float (double-precision)"))
  (bind _output_get (set `self.Health` (`KismetMathLibrary.FClamp` (+ (`self.Health`) HealingAmount) 0.0 100.0)))
  (return _output_get))

(fn `SaveAssaultRifleAmmo`
  (set `self.AssaultRifleAmmo` (`self.GetCurrentAmmo` (`self.AssaultRifle`))))

(fn `SaveShotgunAmmo`
  (set `self.ShotgunAmmo` (`self.GetCurrentAmmo` (`self.Shotgun`))))

(fn `SaveSniperAmmo`
  (set `self.SniperAmmo` (`self.GetCurrentAmmo` (`self.Sniper`))))

(fn `SetBulletDirection`
  (returns (BulletDirection :type "Vector Structure"))
  (bind _output_get (set `self.BulletDirection` (* (`KismetMathLibrary.GetForwardVector` (`self.GetControlRotation`)) (`/Game/Blueprints/Actors/Guns/BP_GunParent.MaxBulletDistance` (`self.EquippedGun`)))))
  (return _output_get))

(fn `SetGunHeat`
  (bind _equippedgun (`self.EquippedGun`))
  (if (`self.IsAlive`)
    (if (`/Game/Blueprints/Actors/Guns/BP_GunParent.IsHeatBased` _equippedgun)
      (`/Game/Blueprints/Actors/Guns/BP_GunParent.HeatUpGun` _equippedgun))))

(fn `ShotgunInInventory`
  (returns (ReturnValue :type Boolean))
  (return (!= (`self.Shotgun`) null)))

(fn `SniperInInventory`
  (returns (ReturnValue :type Boolean))
  (return (!= (`self.Sniper`) null)))

(fn `SpawnAlternativeGun`
  (params (WeaponClass :type "/Game/Blueprints/Actors/Guns/BP_GunParent Class Reference"))
  (`self.K2_DestroyActor` (`self.EquippedGun`))
  (bind _returnvalue (`|SpawnActorFromClass` WeaponClass (`KismetMathLibrary.MakeTransform` (0.0 0.0 0.0)) "Undefined" "OverrideRootScale" null null))
  (bind _output_get (set `self.EquippedGun` _returnvalue))
  (`self.K2_AttachToComponent` _output_get (`self.GunLocation`) "None" "SnapToTarget" "SnapToTarget" "KeepRelative" true))

(fn `SpawnAssaultRifle`
  (bind (_assaultrifleammo_gun _assaultrifleammo_ammocount _assaultrifleammo_maximumammo _assaultrifleammo_currentclip _assaultrifleammo_currentheat) (break `/Game/Blueprints/GunVariables` (`self.AssaultRifleAmmo`)))
  (`self.SpawnAlternativeGun` (`self.AssaultRifle`))
  (`self.LoadSavedAmmo` _assaultrifleammo_ammocount _assaultrifleammo_maximumammo _assaultrifleammo_currentclip _assaultrifleammo_currentheat))

(fn `SpawnPlayerWeapons`
  (bind _returnvalue (`|SpawnActorFromClass` (`self.AssaultRifle`) (`KismetMathLibrary.MakeTransform` (0.0 0.0 0.0)) "Undefined" "OverrideRootScale" null null))
  (bind _output_get (set `self.EquippedGun` _returnvalue))
  (`self.K2_AttachToComponent` _output_get (`self.GunLocation`) "None" "SnapToTarget" "SnapToTarget" "KeepRelative" true))

(fn `SpawnShotgun`
  (bind (_shotgunammo_gun _shotgunammo_ammocount _shotgunammo_maximumammo _shotgunammo_currentclip _shotgunammo_currentheat) (break `/Game/Blueprints/GunVariables` (`self.ShotgunAmmo`)))
  (`self.SpawnAlternativeGun` (`self.Shotgun`))
  (`self.LoadSavedAmmo` _shotgunammo_ammocount _shotgunammo_maximumammo _shotgunammo_currentclip _shotgunammo_currentheat))

(fn `SpawnSniper`
  (bind (_sniperammo_gun _sniperammo_ammocount _sniperammo_maximumammo _sniperammo_currentclip _sniperammo_currentheat) (break `/Game/Blueprints/GunVariables` (`self.SniperAmmo`)))
  (`self.SpawnAlternativeGun` (`self.Sniper`))
  (`self.LoadSavedAmmo` _sniperammo_ammocount _sniperammo_maximumammo _sniperammo_currentclip _sniperammo_currentheat))

(fn `SwitchWeapon`
  (switch `int` (`self.SelectedWeapon`)
    (:`0`
      (if (or (`self.ShotgunInInventory`) (`self.SniperInInventory`))
        (`self.SaveAssaultRifleAmmo`)
        (if (`self.ShotgunInInventory`)
          (`self.SpawnShotgun`)
          (set `self.SelectedWeapon` 1)
          (elif (`self.SniperInInventory`)
            (`self.SpawnSniper`)
            (set `self.SelectedWeapon` 2)))))
    (:`1`
      (if (`self.ShotgunInInventory`)
        (`self.SaveShotgunAmmo`)
        (if (`self.SniperInInventory`)
          (`self.SpawnSniper`)
          (set `self.SelectedWeapon` 2)
          (else
            (`self.SpawnAssaultRifle`)
            (set `self.SelectedWeapon` 0)))))
    (:`2`
      (if (`self.SniperInInventory`)
        (`self.SaveSniperAmmo`)
        (`self.SpawnAssaultRifle`)
        (set `self.SelectedWeapon` 0)))))

(fn `ToggleCameraPosition`
  (params (Alpha :type "Float (double-precision)"))
  (`SceneComponent.K2_SetWorldLocation` (`self.Camera1`) (`KismetMathLibrary.VLerp` (`self.GetCameraStartingLocation`) (`self.Get ADS Location`) Alpha) false false))

(fn `UserConstructionScript`)