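; BP_PlayAreaVolume is a play-area volume that kills the player who stays outside it too long.
; Boundary overlap events set the InPlayArea flag on BP_Ranger.
; Leaving starts a KillPlayer timer of SecondsToPlayerDeath, and re-entering clears it.
; When the timer fires, KillPlayer applies heavy damage to player character 0 rather than the actor that left.
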(event `self.Boundary.OnComponentBeginOverlap`
  (params (OverlappedComponent :type "PrimitiveComponent Object Reference") (OtherActor :type "Actor Object Reference") (OtherComp :type "PrimitiveComponent Object Reference") (OtherBodyIndex :type Integer) (bFromSweep :type Boolean) (SweepResult :type "HitResult Structure (by ref)"))
  (bind _asbp_ranger (cast `/Game/Blueprints/Pawns/BP_Ranger` OtherActor))
  (set `/Game/Blueprints/Pawns/BP_Ranger.InPlayArea` true _asbp_ranger)
  (`KismetSystemLibrary.K2_ClearTimer` null "KillPlayer"))

(event `self.Boundary.OnComponentEndOverlap`
  (params (OverlappedComponent :type "PrimitiveComponent Object Reference") (OtherActor :type "Actor Object Reference") (OtherComp :type "PrimitiveComponent Object Reference") (OtherBodyIndex :type Integer))
  (bind _asbp_ranger (cast `/Game/Blueprints/Pawns/BP_Ranger` OtherActor))
  (set `/Game/Blueprints/Pawns/BP_Ranger.InPlayArea` false _asbp_ranger)
  (`KismetSystemLibrary.K2_SetTimer` null "KillPlayer" (`self.SecondsToPlayerDeath`)))

(fn `KillPlayer`
  (`GameplayStatics.ApplyDamage` (`GameplayStatics.GetPlayerCharacter` 0) 100.0))

(fn `UserConstructionScript`)