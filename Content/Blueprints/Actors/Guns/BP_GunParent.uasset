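; BP_GunParent is a base gun Blueprint that provides hitscan firing with visual and audio feedback.
; FireGun plays the muzzle flash and fire sound attached to the Arrow component, then line-traces the Visibility channel between the supplied start and end locations.
; A blocking hit applies Damage to the hit actor and spawns the same metal impact emitter at the hit location, regardless of surface.
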(fn `FireGun`
  (params (`Start Location` :type "Vector Structure") (`End Location` :type "Vector Structure"))
  (`self.SpawnMuzzleAndSound`)
  (bind _outhit (`KismetSystemLibrary.LineTraceSingle` `Start Location` `End Location` "TraceTypeQuery1"))
  (if (`GameplayStatics.BreakHitResult` _outhit)
    (`GameplayStatics.ApplyDamage` (`.HitActor` (`GameplayStatics.BreakHitResult` _outhit)) (`self.Damage`))
    (`self.SpawnImpact` (`.Location` (`GameplayStatics.BreakHitResult` _outhit)))))

(fn `SpawnImpact`
  (params (Location :type "Vector Structure"))
  (`GameplayStatics.SpawnEmitterAtLocation` "/Game/SciFiWeapLight/FX/Particles/P_Impact_Metal_Medium_Light.P_Impact_Metal_Medium_Light" Location))

(fn `SpawnMuzzleAndSound`
  (bind _arrow (`self.Arrow`))
  (`GameplayStatics.SpawnEmitterAttached` (`self.MuzzleFlashFX`) _arrow "None" (0.0 0.0 0.0) (struct) (0.25 0.25 0.25) "SnapToTarget")
  (`GameplayStatics.SpawnSoundAttached` (`self.GunFireSoundCue`) _arrow "None" (0.0 0.0 0.0) (struct) "KeepRelativeOffset" false 0.4 1.0 0.0 null null))

(fn `UserConstructionScript`)