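; Enemy creature that chases the player, attacks at close range and can be killed.
; BeginPlay re-issues AIMoveTo on each success, while Tick checks range and starts timed attacks that pause movement and apply damage.
; The AttackHand's visibility doubles as the is-attacking flag.
; At zero health it stops, drops collision, increments BP_Ranger's kill count, registers its death with the BP_AntarcticRanger game mode, then destroys itself after a delay.
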(event `self.ReceiveAnyDamage`
  (params (Damage :type "Float (single-precision)") (DamageType :type "DamageType Object Reference") (InstigatedBy :type "Controller Object Reference") (DamageCauser :type "Actor Object Reference"))
  (if (`self.IsAI Alive`)
    (bind _health (`self.DecreaseHealth` Damage))
    (if (== _health 0.0)
      (`self.KillAI`)
      (`KismetSystemLibrary.Delay` 2.0)
      (`self.K2_DestroyActor`))))

(event `self.ReceiveBeginPlay`
  ;[1 1 1] Movement Towards Player
  (if (`self.IsAI Alive`) :!label _label
    (`|AIMoveTo` self (0.0 0.0 0.0) (`GameplayStatics.GetPlayerCharacter` 0)
      (:`OnSuccess`
        (goto _label)))))

(event `self.ReceiveTick`
  (params (DeltaSeconds :type "Float (single-precision)"))
  ;[1 1 1] Attacking The Player
  (if (`self.IsAI Alive`)
    (if (`self.InRangeNotAttacking`)
      (`self.StartAttack`)
      (`KismetSystemLibrary.Delay` 1.0)
      (`self.EndAttack`))))

(fn `Activate AI Movement`
  (`ActorComponent.Activate` (`self.CharacterMovement`) false))

(fn `DamagePlayer`
  (`GameplayStatics.ApplyDamage` (`GameplayStatics.GetPlayerCharacter` 0) (`self.DamagePerHit`)))

(fn `DeactivateAI Movement`
  (`ActorComponent.Deactivate` (`self.CharacterMovement`)))

(fn `DecreaseHealth`
  (params (Damage :type "Float (double-precision)"))
  (returns (Health :type "Float (double-precision)"))
  (bind _output_get (set `self.Health` (`KismetMathLibrary.FClamp` (- (`self.Health`) Damage) 0.0 100.0)))
  (return _output_get))

(fn `EndAttack`
  (`self.HideAttack`)
  (`self.Activate AI Movement`))

(fn `HideAttack`
  (`SceneComponent.SetVisibility` (`self.AttackHand`) false false))

(fn `InRangeNotAttacking`
  (returns (ReturnValue :type Boolean))
  (return (and (`self.IsWithinAttackRange`) (not (`self.IsAttacking`)))))

(fn `IsAI Alive`
  (returns (ReturnValue :type Boolean))
  (return (not (`self.Dead`))))

(fn `IsAttacking`
  (returns (ReturnValue :type Boolean))
  (return (`SceneComponent.IsVisible` (`self.AttackHand`))))

(fn `IsWithinAttackRange`
  (returns (ReturnValue :type Boolean))
  (return (< (`self.GetDistanceTo` (`GameplayStatics.GetPlayerCharacter` 0)) (`self.AttackRange`))))

(fn `KillAI`
  (set `self.Dead` true)
  (`MovementComponent.StopMovementImmediately` (`self.CharacterMovement`))
  (`self.DeactivateAI Movement`)
  (`self.SetActorEnableCollision` false)
  (bind _asbp_ranger (cast `/Game/Blueprints/Pawns/BP_Ranger` (`GameplayStatics.GetPlayerCharacter` 0)))
  (`/Game/Blueprints/Pawns/BP_Ranger.IncreaseKillCount` _asbp_ranger)
  (bind _asbp_antarctic_ranger (cast `/Game/Blueprints/GameModes/BP_AntarcticRanger` (`GameplayStatics.GetGameMode`)))
  (`/Game/Blueprints/GameModes/BP_AntarcticRanger.RegisterEnemyDeath` _asbp_antarctic_ranger self))

(fn `ShowAttack`
  (`SceneComponent.SetVisibility` (`self.AttackHand`) true false))

(fn `StartAttack`
  (`self.DeactivateAI Movement`)
  (`self.ShowAttack`)
  (`self.DamagePlayer`))

(fn `UserConstructionScript`)