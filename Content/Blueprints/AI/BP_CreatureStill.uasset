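; BP_CreatureStill is an enemy AI creature that roams to random reachable points, chases the player's BP_Ranger when seen, and attacks it in melee.
; PawnSensing triggers an AIMoveTo chase, then a timed attack loop halts movement, shows AttackHand and applies damage while the player stays in range.
; Leaving its Box volume clears sight, returning it to roaming after an attack.
; At zero health it stops, turns red, then explodes and is destroyed.
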(event `self.ReceiveAnyDamage`
  (params (Damage :type "Float (single-precision)") (DamageType :type "DamageType Object Reference") (InstigatedBy :type "Controller Object Reference") (DamageCauser :type "Actor Object Reference"))
  (if (`self.IsAI Alive`)
    (bind _health (`self.DecreaseHealth` Damage))
    (if (== _health 0.0)
      (`self.KillAI`)
      (`PrimitiveComponent.SetMaterial` (`self.Body`) 0 "/Game/Materials/M_Red.M_Red")
      (`KismetSystemLibrary.Delay` 2.0)
      (`self.K2_DestroyActor`)
      (`GameplayStatics.SpawnEmitterAtLocation` "/Game/StarterContent/Particles/P_Explosion.P_Explosion" (`self.K2_GetActorLocation`)))))

(event `self.ReceiveBeginPlay`
  ;[1 1 1] Random Roaming
  (`self.Roam`))

(event `Roam`
  ;[1 1 1] Random Roaming
  (`KismetSystemLibrary.Delay` 2.0)
  (`|AIMoveTo` self (`NavigationSystemV1.K2_GetRandomReachablePointInRadius` (`self.K2_GetActorLocation`) 1000.0 null null) null
    (:`OnSuccess`
      (`KismetSystemLibrary.Delay` 2.0)
      (`self.Roam`))))

(event `self.PawnSensing.OnSeePawn`
  (params (Pawn :type "Pawn Object Reference"))
  ;[1 1 1] Chasing and Attacking the Player
  (bind _asbp_ranger (cast `/Game/Blueprints/Pawns/BP_Ranger` Pawn))
  (set `self.CanSeePlayer` true)
  (`|AIMoveTo` self (0.0 0.0 0.0) _asbp_ranger :!label _label
    (:`OnSuccess`
      (`self.StartAttack` :!label _label_2)
      (`KismetSystemLibrary.Delay` 1.0)
      (`self.EndAttack`)
      (`KismetSystemLibrary.Delay` 1.0)
      (if (`self.InRangeNotAttacking`)
        (goto _label_2)
        (elif (`self.CanSeePlayer`)
          (goto _label)
          (else
            (`self.Roam`)))))
    (:`OnFail`
      (set `self.CanSeePlayer` false)
      (`self.Roam`))))

(event `self.Box.OnComponentEndOverlap`
  (params (OverlappedComponent :type "PrimitiveComponent Object Reference") (OtherActor :type "Actor Object Reference") (OtherComp :type "PrimitiveComponent Object Reference") (OtherBodyIndex :type Integer))
  ;[1 1 1] Chasing and Attacking the Player
  (cast `/Game/Blueprints/Pawns/BP_Ranger` OtherActor)
  (set `self.CanSeePlayer` false))

(fn `Activate AI Movement`
  (`ActorComponent.Activate` (`self.CharacterMovement`) false))

(fn `DamagePlayer`
  (`GameplayStatics.ApplyDamage` (`GameplayStatics.GetPlayerCharacter` 0) (`self.DamagePerHit`)))

(fn `DeactivateAI Movement`
  (`ActorComponent.Deactivate` (`self.CharacterMovement`)))

(fn `DecreaseHealth`
  (params (Damage :type "Float (double-precision)"))
  (returns (Health :type "Float (double-precision)"))
  (bind _output_get (set `self.Health` (`KismetMathLibrary.FClamp` (- (`self.Health`) Damage) 0.0 100.0)))
  (return _output_get))

(fn `EndAttack`
  (`self.HideAttack`)
  (`self.Activate AI Movement`))

(fn `HideAttack`
  (`SceneComponent.SetVisibility` (`self.AttackHand`) false false))

(fn `InRangeNotAttacking`
  (returns (ReturnValue :type Boolean))
  (return (and (`self.IsWithinAttackRange`) (not (`self.IsAttacking`)))))

(fn `IsAI Alive`
  (returns (ReturnValue :type Boolean))
  (return (not (`self.Dead`))))

(fn `IsAttacking`
  (returns (ReturnValue :type Boolean))
  (return (`SceneComponent.IsVisible` (`self.AttackHand`))))

(fn `IsWithinAttackRange`
  (returns (ReturnValue :type Boolean))
  (return (< (`self.GetDistanceTo` (`GameplayStatics.GetPlayerCharacter` 0)) (`self.AttackRange`))))

(fn `KillAI`
  (set `self.Dead` true)
  (`MovementComponent.StopMovementImmediately` (`self.CharacterMovement`))
  (`self.DeactivateAI Movement`)
  (`self.SetActorEnableCollision` false))

(fn `ShowAttack`
  (`SceneComponent.SetVisibility` (`self.AttackHand`) true false))

(fn `StartAttack`
  (`self.DeactivateAI Movement`)
  (`self.ShowAttack`)
  (`self.DamagePlayer`))

(fn `UserConstructionScript`)