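; BP_AntarcticRanger is a wave-based game mode that spawns escalating waves of BP_Creature enemies.
; Each wave multiplies the difficulty to set the enemy count, then a looping timer spawns creatures at random TargetPoints until none remain to spawn.
; Spawned enemies are tracked in an array; registered deaths remove them, and an empty array with no spawns left starts the next wave after a short delay.
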(event `self.ReceiveBeginPlay`
  (`KismetSystemLibrary.Delay` 2.0)
  (`self.SetupNewWave`))

(event `Spawn Wave`
  (`self.SpawnEnemy`))

(event `End Wave`
  (`KismetSystemLibrary.Delay` 2.0)
  (`self.SetupNewWave`))

(fn `GetRandomSpawnPoint`
  (returns (SpawnPoint :type "TargetPoint Object Reference"))
  (bind _outactors (`GameplayStatics.GetAllActorsOfClass` "/Script/Engine.TargetPoint"))
  (return (`|GetArrayItem` _outactors (`KismetMathLibrary.RandomIntegerInRange` 0 (`KismetArrayLibrary.Array_LastIndex` _outactors)))))

(fn `IncreaseWaveDifficulty`
  (bind _output_get (set `self.WaveDifficulty` (`KismetMathLibrary.Round` (* (`self.WaveDifficulty`) (`self.DifficultyMultiplier`)))))
  (set `self.EnemySpawnsRemaining` _output_get))

(fn `IsWaveComplete`
  (returns (`Return Value` :type Boolean))
  (return (and (== (`KismetArrayLibrary.Array_Length` (`self.Enemies`)) 0) (== (`self.EnemySpawnsRemaining`) 0))))

(fn `RegisterEnemyDeath`
  (params (Enemy :type "/Game/Blueprints/AI/BP_Creature Object Reference"))
  (`KismetArrayLibrary.Array_RemoveItem` (`self.Enemies`) Enemy)
  (if (`self.IsWaveComplete`)
    (`self.End Wave`)))

(fn `SetupNewWave`
  (`/Engine/EditorBlueprintResources/StandardMacros.IncrementInt` (`self.CurrentWave`)
    (:`  `
      (`self.IncreaseWaveDifficulty`)
      (`KismetSystemLibrary.K2_SetTimer` null "Spawn Wave" (`self.SpawnFrequency`) true))))

(fn `SpawnEnemy`
  (bind _spawnpoint (`self.GetRandomSpawnPoint`))
  (`/Engine/EditorBlueprintResources/StandardMacros.IsValid` _spawnpoint
    (:`Is Valid`
      (bind _returnvalue (`|SpawnActorFromClass` "/Game/Blueprints/AI/BP_Creature.BP_Creature_C" (`self.GetTransform` _spawnpoint) "Undefined" "OverrideRootScale" null null))
      (`/Engine/EditorBlueprintResources/StandardMacros.IsValid` _returnvalue
        (:`Is Valid`
          (`KismetArrayLibrary.Array_Add` (`self.Enemies`) _returnvalue)
          (bind _result (`/Engine/EditorBlueprintResources/StandardMacros.DecrementInt` (`self.EnemySpawnsRemaining`))
            (:`  `
              (if (== _result 0)
                (`KismetSystemLibrary.K2_ClearTimer` null "Spawn Wave")))))))))

(fn `UserConstructionScript`)